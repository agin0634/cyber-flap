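; Obstacle manager that spawns vertical pairs of BP_Shop_Block with randomized height and gap, plus coins.
; While the GM_FC state is Start, Tick spawns one pair, then another whenever the latest block trails the manager by a randomized X distance.
; SpawnCoin randomly adds coins at the pair's midpoint and beside it.
; Restart re-arms the first spawn; the looping timer spawn path is unused.
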(event Custom|CustomEvent_0
  (Utilities|FlowControl|Delay (Math|Random|RandomFloatinRange 1.0 1.5))
  (CallFunction|SpawnBlock))

(event EventBeginPlay
  (bind _asgm_fc (Utilities|Casting|CastToGM_FC (Game|GetGameMode)))
  (Variables|Default|SetGM _asgm_fc))

(event EventTick
  (params (DeltaSeconds :type Float%20%28single-precision%29))
  (switch Utilities|FlowControl|Switch|SwitchonEGameState (Variables|/Game/Blueprint/GM_FC.GM_FC_C|GeteGameState (Variables|Default|GetGM))
    (:NewEnumerator0
      (Utilities|FlowControl|Sequence
        (:then_0
          (Utilities|FlowControl|DoOnce false :!label _label
            (:Completed
              (CallFunction|SpawnBlock))))
        (:then_1
          (Variables|Default|SetOffset (Math|Random|RandomFloatinRange -4e+02 4e+02))
          (if (> (- (.x (Transformation|GetWorldLocation (Variables|Default|GetDefaultSceneRoot))) (.x (Transformation|GetWorldLocation (Variables|/Game/Blueprint/BP_Shop_Block.BP_Shop_Block_C|GetDefaultSceneRoot (Variables|Default|GetCurrentBlock))))) (- 2.4e+03 (Variables|Default|GetOffset)))
            (CallFunction|SpawnBlock)))))
    (:NewEnumerator1
      (goto _label Reset))))

(fn ConstructionScript)

(fn SpawnBlock
  (bind _defaultsceneroot (Variables|Default|GetDefaultSceneRoot))
  (bind _returnvalue (Transformation|GetWorldTransform _defaultsceneroot))
  (bind (_x _y _z) (Math|Vector|BreakVector (.location _returnvalue)))
  ;[1 1 1] Spawn under Block
  (bind _returnvalue_2 (Game|SpawnActorfromClass "/Game/Blueprint/BP_Shop_Block.BP_Shop_Block_C" (Math|Transform|MakeTransform (Math|Vector|MakeVector _x _y (- _z (Math|Random|RandomFloatinRange -5.5e+02 -1.9e+03))) (.rotation _returnvalue) (.scale _returnvalue)) "Undefined" 0 0))
  (LocalVariables|SetUnderBlock _returnvalue_2)
  ;[1 1 1] Spawn Upper Block
  (bind _returnvalue_3 (Game|SpawnActorfromClass "/Game/Blueprint/BP_Shop_Block.BP_Shop_Block_C" (Math|Transform|MakeTransform (Math|Vector|MakeVector (.X (Math|Vector|BreakVector (.location (Transformation|GetWorldTransform (Variables|/Script/Engine.Actor|GetRootComponent (LocalVariables|GetUnderBlock)))))) (.Y (Math|Vector|BreakVector (.location (Transformation|GetWorldTransform (Variables|/Script/Engine.Actor|GetRootComponent (LocalVariables|GetUnderBlock)))))) (- (.Z (Math|Vector|BreakVector (.location (Transformation|GetWorldTransform (Variables|/Script/Engine.Actor|GetRootComponent (LocalVariables|GetUnderBlock)))))) (Math|Random|RandomFloatinRange 2.8e+03 3.3e+03))) (.rotation (Transformation|GetWorldTransform (Variables|/Script/Engine.Actor|GetRootComponent (LocalVariables|GetUnderBlock)))) (.scale (Transformation|GetWorldTransform (Variables|/Script/Engine.Actor|GetRootComponent (LocalVariables|GetUnderBlock))))) "Undefined" 0 0))
  (LocalVariables|SetUpperBlock _returnvalue_3)
  (CallFunction|SpawnCoin (LocalVariables|GetUnderBlock) (LocalVariables|GetUpperBlock))
  (Variables|Default|SetCurrentBlock (LocalVariables|GetUpperBlock)))

(fn SpawnCoin
  (params (UnderBlock :type BP%20Shop%20Block%20Object%20Reference) (UpperBlock :type BP%20Shop%20Block%20Object%20Reference))
  (LocalVariables|SetBlockCenterLocation (/ (+ (Transformation|GetWorldLocation (Variables|/Game/Blueprint/BP_Shop_Block.BP_Shop_Block_C|GetDefaultSceneRoot UnderBlock)) (Transformation|GetWorldLocation (Variables|/Game/Blueprint/BP_Shop_Block.BP_Shop_Block_C|GetDefaultSceneRoot UpperBlock))) 2.0))
  (if (> (Math|Random|RandomIntegerinRange 1 10) 6)
    ;[1 1 1] coin between block
    (Game|SpawnActorfromClass "/Game/Blueprint/BP_Coin.BP_Coin_C" (Math|Transform|MakeTransform (LocalVariables|GetBlockCenterLocation)) "Undefined" 0 0))
  (if (> (Math|Random|RandomIntegerinRange 1 10) 4)
    ;[1 1 1] coin beside block
    (Game|SpawnActorfromClass "/Game/Blueprint/BP_Coin.BP_Coin_C" (Math|Transform|MakeTransform (Math|Vector|MakeVector (+ (.X (Math|Vector|BreakVector (LocalVariables|GetBlockCenterLocation))) (Math|Random|RandomFloatinRange 1e+03 1.3e+03)) (.Y (Math|Vector|BreakVector (LocalVariables|GetBlockCenterLocation))) (Math|Random|RandomFloatinRange -7.5e+02 7.5e+02))) "Undefined" 0 0)))