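; Player actor for a voice-controlled Paper2D game, where microphone loudness drives the sprite up and down.
; BeginPlay finds the BP_AudioCapture actor, caches GM_FC, creates the UI, lists capture devices and requests voice permission.
; Tick branches on game state, mapping the audio envelope to vertical movement and flame flipbooks, resetting on Restart, and showing explosion and lose UI once on Lose.
; A tap during play also jumps the sprite upward.
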(event EventBeginPlay
  (bind _returnvalue (Game|GetPlayerController 0))
  (bind _voicepermission (Variables|Default|GetVoicePermission))
  (Utilities|FlowControl|Sequence
    (:then_0
      (bind _outactors (Actor|GetAllActorsOfClass "/Game/Blueprint/BP_AudioCapture.BP_AudioCapture_C"))
      (Variables|Default|SetAudioCaptureRef (Utilities|Array|Get(acopy) _outactors)))
    (:then_1
      (bind _asgm_fc (Utilities|Casting|CastToGM_FC (Game|GetGameMode)))
      (Variables|Default|SetGM _asgm_fc))
    (:then_2
      (bind _returnvalue_2 (UserInterface|CreateWidget "/Game/Blueprint/W_UI.W_UI_C" _returnvalue))
      (Variables|Default|SetUI _returnvalue_2)
      (UserInterface|Viewport|AddtoViewport _returnvalue_2 0)
      (Input|SetInputModeGameandUI _returnvalue 0 "DoNotLock" false))
    (:then_3
      (bind _outdevices (Class|MediaBlueprintFunctionLibrary|EnumerateAudioCaptureDevices -1))
      (for _array_element _outdevices
        (Development|PrintString (Utilities|String|ToString(Text) (.DisplayName (Utilities|Struct|BreakMediaCaptureDevice _array_element))) true true "(R=0.000000,G=0.660000,B=1.000000,A=1.000000)" 1e+01)))
    (:then_4
      (bind _returnvalue_3 (Class|AndroidPermissionFunctionLibrary|CheckPermission _voicepermission))
      (if (not _returnvalue_3)
        (Class|AndroidPermissionFunctionLibrary|AcquirePermissions (Utilities|Array|MakeArray _voicepermission))))))

(event Collision|EventActorBeginOverlap
  (params (OtherActor :type Actor%20Object%20Reference)))

(event EventTick
  (params (DeltaSeconds :type Float%20%28single-precision%29))
  (bind _audiocaptureref (Variables|Default|GetAudioCaptureRef))
  (bind _speed (Variables|Default|GetSpeed))
  (bind _envelopevalue (Variables|/Game/Blueprint/BP_AudioCapture.BP_AudioCapture_C|GetEnvelopeValue _audiocaptureref))
  (bind _returnvalue (Math|Float|MapRangeClamped _envelopevalue 0.01 0.6 -0.5 1.0))
  (bind _returnvalue_2 (* _returnvalue _speed))
  (switch Utilities|FlowControl|Switch|SwitchonEGameState (Variables|/Game/Blueprint/GM_FC.GM_FC_C|GeteGameState (Variables|Default|GetGM))
    (:NewEnumerator0
      (Transformation|AddLocalOffset (Variables|Default|GetPaperSprite) (Math|Vector|MakeVector 0.0 0.0 _returnvalue_2) false false)
      (if (> _returnvalue_2 0.35)
        (Sprite|SetFlipbook (Variables|Default|Getfront) "/Game/Sprites/Sprites/Fire/fire_2.fire_2")
        (Sprite|SetFlipbook (Variables|Default|Getback) "/Game/Sprites/Sprites/Fire/fire_2.fire_2")
        (else
          (Sprite|SetFlipbook (Variables|Default|Getfront) "/Game/Sprites/Sprites/Fire/fire_1.fire_1")
          (Sprite|SetFlipbook (Variables|Default|Getback) "/Game/Sprites/Sprites/Fire/fire_1.fire_1"))))
    (:NewEnumerator1
      (Transformation|SetWorldLocation (Variables|Default|GetPaperSprite) "0, 0, 0" false false)
      (Sprite|SetFlipbook (Variables|Default|Getexplosion))
      (goto _label Reset))
    (:NewEnumerator2
      (Utilities|FlowControl|DoOnce false :!label _label
        (:Completed
          (Default|ShowLoseUI (Variables|Default|GetUI))
          (Sprite|SetFlipbook (Variables|Default|Getexplosion) "/Game/Sprites/Sprites/explosion/explosion.explosion"))))))

(event Input|ActionEvents|InputActiontap
  (params (Key :type Key%20Structure :default "None"))
  (:Pressed
    (switch Utilities|FlowControl|Switch|SwitchonEGameState (Variables|/Game/Blueprint/GM_FC.GM_FC_C|GeteGameState (Variables|Default|GetGM))
      (:NewEnumerator0
        (Transformation|AddLocalOffset (Variables|Default|GetPaperSprite) (Math|Vector|MakeVector 0.0 0.0 4e+02) false false)))))

(fn ConstructionScript)