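; GM_FC is a game mode Blueprint that tracks the game state, score and coin count.
; Events for begin play, start, restart and lose each set the state enum, with start and restart also zeroing the score.
; On losing, it loads or creates the ScoreData save through SG_SaveData, stores any new high score and caches it in HighScore.
; Coins increment separately and are not saved here.
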(event Custom|AddScore
  ;[1 1 1] Score & Coin
  (bind _result (Math|Integer|IncrementInt (Variables|Default|GetScore))
    (:%20%20
      (Variables|Default|SetScore _result))))

(event Custom|AddCoin
  ;[1 1 1] Score & Coin
  (bind _result (Math|Integer|IncrementInt (Variables|Default|GetCoin))
    (:%20%20
      (Variables|Default|SetCoin _result))))

(event Custom|StartGame
  (Variables|Default|SeteGameState "NewEnumerator0")
  (Variables|Default|SetScore 0))

(event Custom|RestartGame
  (Variables|Default|SeteGameState "NewEnumerator1")
  (Variables|Default|SetScore 0))

(event Custom|LoseGame
  (Variables|Default|SeteGameState "NewEnumerator2")
  (bind _returnvalue (SaveGame|DoesSaveGameExist "ScoreData"))
  (if _returnvalue
    (bind _returnvalue_2 (SaveGame|LoadGamefromSlot "ScoreData"))
    (bind _output_get (Variables|Default|SetSaverSubClass _returnvalue_2))
    (bind _assg_save_data (Utilities|Casting|CastToSG_SaveData _output_get))
    (if (> (Variables|Default|GetScore) (Variables|/Game/Blueprint/SG_SaveData.SG_SaveData_C|GetHighScore _assg_save_data))
      (bind _output_get_2 (Variables|/Game/Blueprint/SG_SaveData.SG_SaveData_C|SetHighScore _assg_save_data (Variables|Default|GetScore)))
      (Variables|Default|SethighScore _output_get_2)
      (SaveGame|SaveGametoSlot (Variables|Default|GetSaverSubClass) "ScoreData")
      (else
        (Variables|Default|SethighScore (Variables|/Game/Blueprint/SG_SaveData.SG_SaveData_C|GetHighScore _assg_save_data))))
    (else
      (bind _returnvalue_3 (SaveGame|CreateSaveGameObject "/Game/Blueprint/SG_SaveData.SG_SaveData_C"))
      (bind _output_get_3 (Variables|Default|SetSaverSubClass _returnvalue_3))
      (bind _assg_save_data_2 (Utilities|Casting|CastToSG_SaveData _output_get_3))
      (bind _output_get_4 (Variables|/Game/Blueprint/SG_SaveData.SG_SaveData_C|SetHighScore _assg_save_data_2 (Variables|Default|GetScore)))
      (Variables|Default|SethighScore _output_get_4)
      (SaveGame|SaveGametoSlot (Variables|Default|GetSaverSubClass) "ScoreData"))))

(event Custom|ResetScore
  ;[1 1 1] Score & Coin
  (Variables|Default|SetScore 0))

(event EventBeginPlay
  (Variables|Default|SeteGameState "NewEnumerator4"))

(fn ConstructionScript)