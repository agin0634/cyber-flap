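; Shop obstacle for a side-scrolling score game, with five Paper2D shop flipbooks picked at random in the construction script.
; While the GM_FC game mode is in Start, it moves along -X by a fixed, frame-rate-dependent step each tick, destroying itself after a set distance or on Restart.
; Overlapping Block loses the game, while leaving the Box trigger adds score and removes that trigger.
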(event OnComponentBeginOverlap(Block)
  (params (OverlappedComponent :type Primitive%20Component%20Object%20Reference) (OtherActor :type Actor%20Object%20Reference) (OtherComp :type Primitive%20Component%20Object%20Reference) (OtherBodyIndex :type Integer) (bFromSweep :type Boolean) (SweepResult :type Hit%20Result%20Structure%20%28by%20ref%29))
  (Default|LoseGame (Variables|Default|GetGM)))

(event OnComponentEndOverlap(Box)
  (params (OverlappedComponent :type Primitive%20Component%20Object%20Reference) (OtherActor :type Actor%20Object%20Reference) (OtherComp :type Primitive%20Component%20Object%20Reference) (OtherBodyIndex :type Integer))
  (Default|AddScore (Variables|Default|GetGM))
  (Components|DestroyComponent (Variables|Default|GetBox)))

(event EventBeginPlay
  (bind _asgm_fc (Utilities|Casting|CastToGM_FC (Game|GetGameMode)))
  (Variables|Default|SetGM _asgm_fc)
  (Variables|Default|SetPreviousLocation (Transformation|GetWorldLocation (Variables|Default|GetDefaultSceneRoot))))

(event Collision|EventActorBeginOverlap
  (params (OtherActor :type Actor%20Object%20Reference)))

(event EventTick
  (params (DeltaSeconds :type Float%20%28single-precision%29))
  (switch Utilities|FlowControl|Switch|SwitchonEGameState (Variables|/Game/Blueprint/GM_FC.GM_FC_C|GeteGameState (Variables|Default|GetGM))
    (:NewEnumerator0
      (Transformation|AddLocalOffset (Variables|Default|GetDefaultSceneRoot) (Math|Vector|MakeVector -5.0 0.0 0.0) false false)
      (if (> (- (.x (Variables|Default|GetPreviousLocation)) (.x (Transformation|GetWorldLocation (Variables|Default|GetDefaultSceneRoot)))) 6e+03)
        (Actor|DestroyActor)))
    (:NewEnumerator1
      (Utilities|FlowControl|DoOnce false
        (:Completed
          (Actor|DestroyActor))))))

(fn ConstructionScript
  (bind _returnvalue (Math|Random|RandomIntegerinRange 0 4))
  (bind _block_styles_anim (Variables|Default|GetBlock_Styles_anim))
  (bind _output (Utilities|Array|Get(acopy) _block_styles_anim _returnvalue))
  (Sprite|SetFlipbook (Variables|Default|GetShop1) _output)
  (Sprite|SetFlipbook (Variables|Default|GetShop2) _output)
  (Sprite|SetFlipbook (Variables|Default|GetShop3) _output)
  (Sprite|SetFlipbook (Variables|Default|GetShop4) _output)
  (Sprite|SetFlipbook (Variables|Default|GetShop5) _output))